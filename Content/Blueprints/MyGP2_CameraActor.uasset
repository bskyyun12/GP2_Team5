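; MyGP2_CameraActor is a camera actor that follows the player character.
; On BeginPlay it finds the GP2_Team5Character in the level, caches it as PlayerActor and prints its name, or an error if none is found.
; Each Tick passes that actor with the Zoom and CameraSpeed values to FollowActor, whose logic is defined outside these graphs.
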(event EventBeginPlay
  (bind _returnvalue (Actor|GetActorOfClass "/Script/GP2_Team5.GP2_Team5Character"))
  (Utilities|IsValid 0
    (:Is%20Valid
      (bind _output_get (Variables|Default|SetPlayerActor _returnvalue))
      (Development|PrintString (Utilities|GetDisplayName _output_get)))
    (:Is%20Not%20Valid
      (Development|PrintString "Player Actor not found/null!"))))

(event Collision|EventActorBeginOverlap
  (params (OtherActor :type Actor%20Object%20Reference)))

(event EventTick
  (params (DeltaSeconds :type Float%20%28single-precision%29))
  (Class|GP2CameraActor|FollowActor (Variables|Default|GetPlayerActor) (Variables|Default|GetZoom) (Variables|Default|GetCameraSpeed)))

(fn ConstructionScript)
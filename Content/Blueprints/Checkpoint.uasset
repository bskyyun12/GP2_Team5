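; Checkpoint trigger actor that writes to a BP_SaveGameScript save when anything overlaps its TriggerBox.
; With LoadNewLevel true, it stores the player's location and sets LoadGame, updating the existing save or creating one.
; Otherwise it only sets LoadGame to true on the loaded save, despite printing "Save state cleared!".
; The existence check uses slot "Check", while saves use the SaveGameSlot variable.
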(event OnComponentBeginOverlap(TriggerBox)
  (params (OverlappedComponent :type Primitive%20Component%20Object%20Reference) (OtherActor :type Actor%20Object%20Reference) (OtherComp :type Primitive%20Component%20Object%20Reference) (OtherBodyIndex :type Integer) (bFromSweep :type Boolean) (SweepResult :type Hit%20Result%20Structure%20%28by%20ref%29))
  (if (Variables|Default|GetLoadNewLevel)
    (Utilities|FlowControl|Sequence
      (:then_0
        (bind _asgravity_player_character (Utilities|Casting|CastToGravityPlayerCharacter (Game|GetPlayerCharacter 0)))
        (Variables|Default|SetLocalPlayerLoc (Transformation|GetActorLocation _asgravity_player_character)))
      (:then_1
        (bind _returnvalue (SaveGame|DoesSaveGameExist "Check"))
        (if _returnvalue
          (bind _returnvalue_2 (SaveGame|LoadGamefromSlot (Variables|Default|GetSaveGameSlot)))
          (bind _asbp_save_game_script (Utilities|Casting|CastToBP_SaveGameScript _returnvalue_2))
          (Variables|/Game/Blueprints/BP_SaveGameScript.BP_SaveGameScript_C|SetPlayerLocation _asbp_save_game_script (Variables|Default|GetLocalPlayerLoc))
          (Variables|/Game/Blueprints/BP_SaveGameScript.BP_SaveGameScript_C|SetLoadGame _asbp_save_game_script true)
          (SaveGame|SaveGametoSlot _asbp_save_game_script (Variables|Default|GetSaveGameSlot))
          (else
            (bind _returnvalue_3 (SaveGame|CreateSaveGameObject "/Game/Blueprints/BP_SaveGameScript.BP_SaveGameScript_C"))
            (Variables|/Game/Blueprints/BP_SaveGameScript.BP_SaveGameScript_C|SetPlayerLocation _returnvalue_3 (Variables|Default|GetLocalPlayerLoc))
            (Variables|/Game/Blueprints/BP_SaveGameScript.BP_SaveGameScript_C|SetLoadGame _returnvalue_3 true)
            (SaveGame|SaveGametoSlot _returnvalue_3 (Variables|Default|GetSaveGameSlot))
            (Development|PrintString "Made a new save state!")))))
    (else
      (bind _returnvalue_4 (SaveGame|LoadGamefromSlot "SaveGameSlot"))
      (bind _asbp_save_game_script_2 (Utilities|Casting|CastToBP_SaveGameScript _returnvalue_4))
      (Variables|/Game/Blueprints/BP_SaveGameScript.BP_SaveGameScript_C|SetLoadGame _asbp_save_game_script_2 true)
      (SaveGame|SaveGametoSlot _asbp_save_game_script_2 (Variables|Default|GetSaveGameSlot))
      (Development|PrintString "Save state cleared!"))))

(event EventBeginPlay)

(event Collision|EventActorBeginOverlap
  (params (OtherActor :type Actor%20Object%20Reference)))

(event EventTick
  (params (DeltaSeconds :type Float%20%28single-precision%29)))

(fn ConstructionScript)
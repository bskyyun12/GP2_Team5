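; Base puzzle actor with a toggleable outline highlight, click-toggled temporary point light and gravity-flip response.
; BeginPlay adds a hidden, collisionless mesh copy with dynamic MI_Outline materials, setting color and scale only on the last instance.
; ShowOutline and HideOutline toggle that copy, while ClickInteract events toggle or reset the light.
; Gravity flips pause mesh physics for FlipDelay; approach-grab handlers are empty.
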(event OnClickInteract(ClickInteract)
  (bind _output_get (Variables|Default|SetbLightOn (not (Variables|Default|GetbLightOn))))
  (Rendering|SetVisibility (Variables|Default|GetTempPointLight) _output_get false))

(event OnResetClickInteract(ClickInteract)
  (bind _output_get (Variables|Default|SetbLightOn false))
  (Rendering|SetVisibility (Variables|Default|GetTempPointLight) _output_get false))

(event OnInteract(BP_ApproachGrabComponent))

(event OnInteractReleased(BP_ApproachGrabComponent))

(event OnFlipGravity(GravitySwap)
  (params (bInverted :type Boolean))
  (Physics|SetSimulatePhysics (Variables|Default|GetStaticMesh) false)
  (Utilities|FlowControl|Delay (Variables|Default|GetFlipDelay))
  (Physics|SetSimulatePhysics (Variables|Default|GetStaticMesh) true))

(event EventHideOutline
  (bind _meshcomp (Variables|Default|GetMeshComp))
  ;[1 1 1] Outline On and Off
  (Utilities|IsValid _meshcomp
    (:Is%20Valid
      (Rendering|SetVisibility _meshcomp false false))))

(event EventShowOutline
  (bind _meshcomp (Variables|Default|GetMeshComp))
  ;[1 1 1] Outline On and Off
  (Utilities|IsValid _meshcomp
    (:Is%20Valid
      (Rendering|SetVisibility _meshcomp true false))))

(event EventBeginPlay
  ;[1 1 1] Outline setup
  (Utilities|FlowControl|Sequence
    (:then_0
      ;[1 1 1] Temporary Light setup
      (Rendering|SetVisibility (Variables|Default|GetTempPointLight) (Variables|Default|GetbLightOn) false))
    (:then_1
      (Components|StaticMesh|SetStaticMesh (Variables|Default|GetStaticMesh) (Variables|Default|GetMesh))
      (bind _returnvalue (AddComponent|AddStaticMeshComponent true (Transformation|GetWorldTransform (Variables|Default|GetStaticMesh))))
      (bind _output_get (Variables|Default|SetMeshComp _returnvalue))
      (Transformation|AttachComponentToComponent _output_get (Variables|Default|GetStaticMesh) "None" "KeepWorld" "KeepWorld" "KeepWorld" true)
      (Collision|SetCollisionEnabled _output_get "NoCollision")
      (Rendering|SetVisibility _output_get false false)
      (Components|StaticMesh|SetStaticMesh _output_get (Variables|Default|GetMesh))
      (for (_ _array_index) (Rendering|Material|GetMaterials _output_get)
        (bind _returnvalue_2 (Rendering|Material|CreateDynamicMaterialInstance _output_get _array_index "/Game/T5_PuzzleGame/Maps/Gwangyeong/MI_Outline.MI_Outline" "None" :!class /Script/Engine.PrimitiveComponent)))
      (Rendering|Material|SetVectorParameterValue _returnvalue_2 "color" (Variables|Default|GetOutlineColor) :!class /Script/Engine.MaterialInstanceDynamic)
      (Rendering|Material|SetScalarParameterValue _returnvalue_2 "Scale" (Variables|Default|GetOutlineScale) :!class /Script/Engine.MaterialInstanceDynamic))))

(fn ConstructionScript)
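; BP_MouseOverEventComp is a component for the puzzle game that reacts to the mouse cursor entering and leaving its owner's static mesh.
; On BeginPlay it binds to the cursor-over events of the owner's StaticMeshComponent.
; Those handlers forward to BeginCursorOver and EndCursorOver events, which currently only print the component name with "Outliner On" or "Outliner Off" as placeholder highlight feedback.
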(event Custom|OnBeginCursorOver
  (params (TouchedComponent :type Primitive%20Component%20Object%20Reference))
  (CallFunction|BeginCursorOver TouchedComponent))

(event Custom|OnEndCursorOver
  (params (TouchedComponent :type Primitive%20Component%20Object%20Reference))
  (CallFunction|EndCursorOver TouchedComponent))

(event Custom|EndCursorOver
  (params (TouchedComp :type Primitive%20Component%20Object%20Reference))
  (Development|PrintString (Utilities|String|Append (Utilities|GetDisplayName TouchedComp) ": Outliner Off")))

(event Custom|BeginCursorOver
  (params (TouchedComp :type Primitive%20Component%20Object%20Reference))
  (Development|PrintString (Utilities|String|Append (Utilities|GetDisplayName TouchedComp) ": Outliner On")))

(event EventBeginPlay
  (bind _returnvalue (Components|GetOwner))
  (bind _returnvalue_2 (Actor|GetComponentbyClass _returnvalue "/Script/Engine.StaticMeshComponent"))
  (EventDispatchers|AssignOnBeginCursorOver _returnvalue_2 (delegate Custom|OnBeginCursorOver))
  (EventDispatchers|BindEventtoOnEndCursorOver _returnvalue_2 (delegate Custom|OnEndCursorOver)))

(event EventTick
  (params (DeltaSeconds :type Float%20%28single-precision%29)))
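; Base character for a gravity puzzle game that supports flipping gravity and click-highlight interaction.
; On begin play it applies its starting gravity, and GravitySwap flip events negate or restore the camera boom's socket offset.
; A temporary light is recolored every tick to show gravity state.
; ClickInteract events show a colored highlight light, hiding it on deactivation unless the character has click focus and is still clickable.
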(event OnFlipGravity(GravitySwap)
  (params (bInverted :type Boolean))
  (bind _cameraboom (Variables|Default|GetCameraBoom))
  (bind _cameraboomdefaultoffset (Variables|Default|GetCameraBoomDefaultOffset))
  ;[1 1 1] On Flip Gravity :  Change camera focus when gravity flips
  (bind _output_get (Variables|Default|SetbFlipGravity bInverted))
  (if _output_get
    (Variables|/Script/Engine.SpringArmComponent|SetSocketOffset _cameraboom (* _cameraboomdefaultoffset -1.0))
    (else
      (Variables|/Script/Engine.SpringArmComponent|SetSocketOffset _cameraboom _cameraboomdefaultoffset))))

(event OnActivateHighlight(ClickInteract)
  (params (bIsWithinRange :type Boolean) (HightlightColor :type Color%20Structure))
  ;[1 1 1] Show highlight
  (Rendering|SetVisibility (Variables|Default|GetTempClickedLight) true false)
  (Rendering|Components|Light|SetLightColor (Variables|Default|GetTempClickedLight) (Math|Conversions|ToLinearColor(Color) HightlightColor) true))

(event OnDeactivateHighlight(ClickInteract)
  (params (bIsWithinRange :type Boolean) (bClickable :type Boolean))
  ;[1 1 1] Hide highlight
  (if (Class|GravityCharacter|HasCurrentClickFocus) ; Player has current focus?
    (if (not bClickable) ; Is player clickable?
      (Rendering|SetVisibility (Variables|Default|GetTempClickedLight) false false :!label _label))
    (else
      (goto _label))))

(event EventBeginPlay
  (Class|GravityCharacter|SetGravityTarget (Variables|Default|GetStartGravity))
  (Variables|Default|SetCameraBoomDefaultOffset (Variables|/Script/Engine.SpringArmComponent|GetSocketOffset (Variables|Default|GetCameraBoom))))

(event EventTick
  (params (DeltaSeconds :type Float%20%28single-precision%29))
  ;[1 1 1] Temporary stuff
  (if (Variables|Default|GetbFlipGravity)
    (Rendering|Components|Light|SetLightColor (Variables|Default|GetTempCharacterLight) (Variables|Default|GetTempBlueColor) true)
    (else
      (Rendering|Components|Light|SetLightColor (Variables|Default|GetTempCharacterLight) (Variables|Default|GetTempRedColor) true))))

(fn ConstructionScript)
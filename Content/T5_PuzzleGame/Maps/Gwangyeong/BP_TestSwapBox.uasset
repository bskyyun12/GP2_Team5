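; Test puzzle box actor with click-interact, gravity-swap and grab components; grab interaction only prints a debug string.
; Highlighting swaps in a dynamic outline material, also added as a post-process blendable, and sets custom depth stencil by highlight type.
; Highlight clears unless the player has click focus and the box is in range and clickable.
; Gravity flips pause physics for a delay, and a helper sets four capsules' collision response.
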(event OnClickInteract(ClickInteract))

(event OnResetClickInteract(ClickInteract))

(event OnInteract(BP_ApproachGrabComponent)
  (Development|PrintString "Hello"))

(event OnInteractReleased(BP_ApproachGrabComponent))

(event OnFlipGravity(GravitySwap)
  (params (bInverted :type Boolean))
  ;[1 1 1] On Flip Gravity
  (Physics|SetSimulatePhysics (Variables|Default|GetStaticMesh) false)
  (Utilities|FlowControl|Delay (Variables|Default|GetFlipDelay))
  (Physics|SetSimulatePhysics (Variables|Default|GetStaticMesh) true))

(event OnActivateHighlight(ClickInteract)
  (params (bIsWithinRange :type Boolean) (HightlightType :type EHighlightType%20Enum :default "Hover"))
  (bind _staticmesh (Variables|Default|GetStaticMesh))
  ;[1 1 1] Show highlight
  (Rendering|Material|SetMaterial (Variables|Default|GetStaticMesh) 0 (Variables|Outline|GetDynamicMat))
  (Rendering|SetRenderCustomDepth (Variables|Default|GetStaticMesh) true)
  (switch Utilities|FlowControl|Switch|SwitchonEHighlightType HightlightType
    (:Hover
      (Rendering|SetCustomDepthStencilValue _staticmesh 0))
    (:Swappable
      (Rendering|SetCustomDepthStencilValue _staticmesh 1))
    (:NonClickable
      (Rendering|SetCustomDepthStencilValue _staticmesh 2))))

(event OnDeactivateHighlight(ClickInteract)
  (params (bIsWithinRange :type Boolean) (bClickable :type Boolean))
  ;[1 1 1] Hide highlight
  (bind _asbp_gravity_character_base (Utilities|Casting|CastToBP_GravityCharacterBase (Game|GetPlayerCharacter 0)))
  (if (Class|GravityCharacter|HasCurrentClickFocus _asbp_gravity_character_base) ; Player has current focus?
    (if bIsWithinRange ; Within interact range?
      (if (not bClickable) ; Is this clickable?
        (Rendering|Material|SetMaterial (Variables|Default|GetStaticMesh) 0 (Variables|Outline|GetDefaultMat) :!label _label)
        (Rendering|SetRenderCustomDepth (Variables|Default|GetStaticMesh) false))
      (else
        (goto _label)))
    (else
      (goto _label))))

(event EventBeginPlay
  ;[1 1 1] BeginPlay
  (bind _returnvalue (Rendering|Material|CreateDynamicMaterialInstance (Variables|Outline|GetOutlineMat) "None" :!class /Script/Engine.KismetMaterialLibrary))
  (bind _output_get (Variables|Outline|SetDynamicMat _returnvalue))
  (Rendering|AddorUpdateBlendable (Variables|Default|GetPostProcess) _output_get 1.0 :!class /Script/Engine.PostProcessComponent)
  (Variables|Outline|SetDefaultMat (Rendering|Material|GetMaterial (Variables|Default|GetStaticMesh) 0)))

(fn ConstructionScript)

(fn SetGrondCollision
  (params (CollisionEnabled :type ECollisionResponse%20Enum :default "ECR_Ignore"))
  (Collision|SetCollisionResponsetoChannel (Variables|Default|GetCapsule) "ECC_GameTraceChannel2" CollisionEnabled))
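; Actor that shuttles back and forth along the MyySpline component of a referenced spline actor (Spline1Ref), following its location and rotation.
; On BeginPlay, two timelines get play rates of 1/Duration; their Alpha maps to distance along the spline in world space.
; SplineMover drives the outward trip and a second timeline plays in reverse for the return, with a one-second pause at each end, looping indefinitely.
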(event EventBeginPlay
  (Components|Timeline|SetPlayRate (Variables|Default|GetSplineMover) (/ 1.0 (Variables|Default|GetDuration)))
  (Components|Timeline|SetPlayRate (Variables|Default|GetTimeline_0) (/ 1.0 (Variables|Default|GetDuration)))
  (bind _alpha (Timeline|SplineMover Play)
    (:Update
      (Variables|Default|SetAlpha _alpha)
      (Transformation|SetActorLocationAndRotation (Spline|GetLocationatDistanceAlongSpline (Variables|/Game/T5_PuzzleGame/Maps/Gwangyeong/BP_Spline1.BP_Spline1_C|GetMyySpline (Variables|Default|GetSpline1Ref)) (Math|Float|Lerp 0.0 (Spline|GetSplineLength (Variables|/Game/T5_PuzzleGame/Maps/Gwangyeong/BP_Spline1.BP_Spline1_C|GetMyySpline (Variables|Default|GetSpline1Ref))) (Variables|Default|GetAlpha)) "World") (Spline|GetRotationatDistanceAlongSpline (Variables|/Game/T5_PuzzleGame/Maps/Gwangyeong/BP_Spline1.BP_Spline1_C|GetMyySpline (Variables|Default|GetSpline1Ref)) (Math|Float|Lerp 0.0 (Spline|GetSplineLength (Variables|/Game/T5_PuzzleGame/Maps/Gwangyeong/BP_Spline1.BP_Spline1_C|GetMyySpline (Variables|Default|GetSpline1Ref))) (Variables|Default|GetAlpha)) "World")))
    (:Finished
      (Utilities|FlowControl|Delay 1.0)
      (bind _alpha_2 (Timeline|Timeline_0 ReverseFromEnd)
        (:Update
          (Variables|Default|SetAlpha _alpha_2)
          (Transformation|SetActorLocationAndRotation (Spline|GetLocationatDistanceAlongSpline (Variables|/Game/T5_PuzzleGame/Maps/Gwangyeong/BP_Spline1.BP_Spline1_C|GetMyySpline (Variables|Default|GetSpline1Ref)) (Math|Float|Lerp 0.0 (Spline|GetSplineLength (Variables|/Game/T5_PuzzleGame/Maps/Gwangyeong/BP_Spline1.BP_Spline1_C|GetMyySpline (Variables|Default|GetSpline1Ref))) (Variables|Default|GetAlpha)) "World") (Spline|GetRotationatDistanceAlongSpline (Variables|/Game/T5_PuzzleGame/Maps/Gwangyeong/BP_Spline1.BP_Spline1_C|GetMyySpline (Variables|Default|GetSpline1Ref)) (Math|Float|Lerp 0.0 (Spline|GetSplineLength (Variables|/Game/T5_PuzzleGame/Maps/Gwangyeong/BP_Spline1.BP_Spline1_C|GetMyySpline (Variables|Default|GetSpline1Ref))) (Variables|Default|GetAlpha)) "World")))
        (:Finished
          (Utilities|FlowControl|Delay 1.0)
          (Timeline|SplineMover PlayFromStart))))))

(fn ConstructionScript)
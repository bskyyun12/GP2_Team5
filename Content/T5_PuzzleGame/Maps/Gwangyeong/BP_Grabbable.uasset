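; BP_Grabbable is a puzzle object that toggles IsGrabbed on interact and snaps in front of player 0 when grabbed.
; A trace toward world origin, or radially outward when GravitySwap is unflipped, aligns it to the surface normal and sets height.
; Grabbing disables physics, ignores a custom channel on four capsules and stops GravityCharacter orienting to movement.
; The restoring branch is nested under the grabbed check, so releasing only clears the flag.
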(event OnInteract(ApproachInteract)
  (bind _returnvalue (Transformation|GetActorRotation))
  (bind _returnvalue_2 (Game|GetPlayerCharacter 0))
  (bind _returnvalue_3 (Game|GetPlayerCharacter 0))
  (bind _rootcomponent (Variables|Transformation|GetRootComponent))
  (bind _staticmesh (Variables|Default|GetStaticMesh))
  (bind _rootcomponent_2 (Variables|Transformation|GetRootComponent))
  (bind _returnvalue_4 (Transformation|GetWorldLocation _staticmesh))
  (bind (_roll _pitch _yaw) (Math|Rotator|BreakRotator _returnvalue))
  (bind _capsulecomponent (Variables|/Script/Engine.Character|GetCapsuleComponent _returnvalue_2))
  (bind _capsulecomponent_2 (Variables|/Script/Engine.Character|GetCapsuleComponent _returnvalue_3))
  (bind _returnvalue_5 (Transformation|GetWorldLocation _capsulecomponent_2))
  (bind _returnvalue_6 (Math|Vector|GetForwardVector _capsulecomponent))
  (bind _returnvalue_7 (Transformation|GetWorldLocation _capsulecomponent))
  (bind _returnvalue_8 (Math|Vector|GetForwardVector _capsulecomponent_2))
  (bind _returnvalue_9 (* _returnvalue_8 1.2e+02))
  (bind _returnvalue_10 (* _returnvalue_6 1.2e+02))
  (bind _returnvalue_11 (+ _returnvalue_5 _returnvalue_9))
  (bind _returnvalue_12 (+ _returnvalue_7 _returnvalue_10))
  (bind _output_get (Variables|Default|SetbIsGrabbed (not (Variables|Default|GetbIsGrabbed))))
  (if _output_get
    (if (Variables|/Script/GP2_Team5.GravitySwapComponent|GetbFlipGravity (Variables|Default|GetGravitySwap))
      (bind _outhit (Collision|LineTraceByChannel (Transformation|GetWorldLocation (Variables|Default|GetStaticMesh)) "0, 0, 0" "TraceTypeQuery1" false 0 "ForOneFrame"))
      (Transformation|SetWorldRotation _rootcomponent_2 (Math|Rotator|MakeRotfromZX (.ImpactNormal (Collision|BreakHitResult _outhit)) (Math|Vector|GetForwardVector (Math|Rotator|MakeRotator _roll 0.0 _yaw))) false false)
      (Transformation|SetWorldLocation _rootcomponent_2 (- _returnvalue_11 (* (Math|Vector|GetUpVector (Variables|Default|GetStaticMesh)) (- (Math|Vector|Distance(Vector) _returnvalue_11 (.ImpactPoint (Collision|BreakHitResult _outhit))) 65.0))) true false)
      (else
        (bind _outhit_2 (Collision|LineTraceByChannel _returnvalue_4 (* (Math|Vector|GetUnitDirection(Vector) "0, 0, 0" _returnvalue_4) 1e+04) "TraceTypeQuery1" false 0 "ForOneFrame"))
        (Transformation|SetWorldRotation _rootcomponent (Math|Rotator|MakeRotfromZX (.ImpactNormal (Collision|BreakHitResult _outhit_2)) (Math|Vector|GetForwardVector (Variables|/Script/Engine.Character|GetCapsuleComponent (Game|GetPlayerCharacter 0)))) false false)
        (Transformation|SetWorldLocation _rootcomponent (- _returnvalue_12 (* (Math|Vector|GetUpVector (Variables|Default|GetStaticMesh)) (- (Math|Vector|Distance(Vector) _returnvalue_12 (.ImpactPoint (Collision|BreakHitResult _outhit_2))) 65.0))) true false)))
    (if (Variables|Default|GetbIsGrabbed)
      (Collision|SetCollisionResponsetoChannel (Variables|Default|GetCapsule) "ECC_GameTraceChannel2" "ECR_Ignore")
      (Physics|SetSimulatePhysics (Variables|Default|GetStaticMesh) false)
      (bind _asgravity_character (Utilities|Casting|CastToGravityCharacter (Game|GetPlayerCharacter 0)))
      (Variables|/Script/Engine.CharacterMovementComponent|SetbOrientRotationToMovement (Class|GravityCharacter|GetGravityMovementComponent _asgravity_character) false)
      (else
        (Collision|SetCollisionResponsetoChannel (Variables|Default|GetCapsule2) "ECC_GameTraceChannel2" "ECR_Block")
        (Physics|SetSimulatePhysics (Variables|Default|GetStaticMesh) true)
        (bind _asgravity_character_2 (Utilities|Casting|CastToGravityCharacter (Game|GetPlayerCharacter 0)))
        (Variables|/Script/Engine.CharacterMovementComponent|SetbOrientRotationToMovement (Class|GravityCharacter|GetGravityMovementComponent _asgravity_character_2) true)))))

(event EventBeginPlay)

(event Collision|EventActorBeginOverlap
  (params (OtherActor :type Actor%20Object%20Reference)))

(event EventTick
  (params (DeltaSeconds :type Float%20%28single-precision%29)))

(fn ConstructionScript)
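; Puzzle-game destructible prop that shatters when a BP_GravitySwappablePushBox enters its Box trigger.
; At BeginPlay it assigns its configured mesh to the Destructible component and hides the StaticMesh.
; On overlap it waits briefly, applies heavy damage and impulse at the push box's location, then destroys itself a few seconds later.
; The impulse direction is simply the box's world position vector, not relative to the prop.
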(event OnComponentBeginOverlap(Box)
  (params (OverlappedComponent :type Primitive%20Component%20Object%20Reference) (OtherActor :type Actor%20Object%20Reference) (OtherComp :type Primitive%20Component%20Object%20Reference) (OtherBodyIndex :type Integer) (bFromSweep :type Boolean) (SweepResult :type Hit%20Result%20Structure%20%28by%20ref%29))
  (bind _returnvalue (Transformation|GetActorLocation OtherActor))
  (bind _asbp_gravity_swappable_push_box (Utilities|Casting|CastToBP_GravitySwappablePushBox OtherActor))
  (Utilities|FlowControl|Delay 0.2)
  (Class|DestructibleComponent|ApplyDamage (Variables|Default|GetDestructible) 5555.0 _returnvalue (- _returnvalue (Math|Vector|VectorZero)) 5555.0)
  (Utilities|FlowControl|Delay 3.0)
  (Actor|DestroyActor))

(event EventBeginPlay
  (Class|DestructibleComponent|SetDestructibleMesh (Variables|Default|GetDestructible) (Variables|Default|GetDestructableMesh))
  (Rendering|SetVisibility (Variables|Default|GetStaticMesh) false false))

(fn ConstructionScript)
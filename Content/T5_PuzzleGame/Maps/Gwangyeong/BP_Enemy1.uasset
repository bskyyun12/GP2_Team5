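; BP_Enemy1 is an enemy in the puzzle game whose movement is constrained to a spline path.
; On BeginPlay, after the parent logic, it teleports its capsule to the closest point on Spline1's spline.
; Every Tick it snaps the capsule back to the nearest spline point, without sweep or teleport.
; The parent Tick call is disconnected, so only the snapping runs per frame.
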(event EventBeginPlay
  (|CallParentFunction)
  (Transformation|SetWorldLocation (Variables|Default|GetCapsuleComponent) (Spline|FindLocationClosesttoWorldLocation (Variables|/Game/T5_PuzzleGame/Maps/Gwangyeong/BP_Spline1.BP_Spline1_C|GetMyySpline (Variables|Default|GetSpline1)) (Transformation|GetWorldLocation (Variables|Default|GetCapsuleComponent)) "World") false true))

(event Collision|EventActorBeginOverlap
  (params (OtherActor :type Actor%20Object%20Reference))
  (|CallParentFunction OtherActor) ; This node is disabled and will not be called.\nDrag off pins to build functionality.
)

(event EventTick
  (params (DeltaSeconds :type Float%20%28single-precision%29))
  (Transformation|SetWorldLocation (Variables|Default|GetCapsuleComponent) (Spline|FindLocationClosesttoWorldLocation (Variables|/Game/T5_PuzzleGame/Maps/Gwangyeong/BP_Spline1.BP_Spline1_C|GetMyySpline (Variables|Default|GetSpline1)) (Transformation|GetWorldLocation (Variables|Default|GetCapsuleComponent)) "World") false false))

(fn ConstructionScript
  (|CallParentFunction))
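; BP_DestructableActor is a puzzle-game placeable that shatters when a fast-moving big rock push box hits it.
; At BeginPlay it assigns the destructible mesh and hides the static mesh, whose collision is disabled on breaking.
; Box overlap checks the rock's exact class and speed, briefly delays, applies heavy damage and impulse, then destroys the actor seconds later.
; The impulse direction is the rock's world position, not its velocity.
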(event OnComponentBeginOverlap(Box)
  (params (OverlappedComponent :type Primitive%20Component%20Object%20Reference) (OtherActor :type Actor%20Object%20Reference) (OtherComp :type Primitive%20Component%20Object%20Reference) (OtherBodyIndex :type Integer) (bFromSweep :type Boolean) (SweepResult :type Hit%20Result%20Structure%20%28by%20ref%29))
  (bind _returnvalue (Transformation|GetActorLocation OtherActor))
  (if (== (Utilities|GetClass OtherActor) "/Game/T5_PuzzleGame/Placeables/Interactables/BP_GravitySwappablePushBox_Big_Rock.BP_GravitySwappablePushBox_Big_Rock_C")
    (if (> (Math|Vector|VectorLength (Transformation|GetVelocity OtherActor)) 1e+03)
      (Utilities|FlowControl|Delay 0.1)
      (Class|DestructibleComponent|ApplyDamage (Variables|Default|GetDestructible) 5555.0 _returnvalue (- _returnvalue (Math|Vector|VectorZero)) 5555.0)
      (Collision|SetCollisionEnabled (Variables|Default|GetStaticMesh) "NoCollision")
      (Utilities|FlowControl|Delay 3.0)
      (Actor|DestroyActor))))

(event EventBeginPlay
  (Class|DestructibleComponent|SetDestructibleMesh (Variables|Default|GetDestructible) (Variables|Default|GetDestructableMesh))
  (Rendering|SetVisibility (Variables|Default|GetStaticMesh) false false))

(fn ConstructionScript)
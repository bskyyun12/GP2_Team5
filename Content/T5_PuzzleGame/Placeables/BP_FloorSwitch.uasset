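; Floor switch placeable for a puzzle game on a spherical world, aligned to the sphere at construction with an optional upside-down flag.
; A box overlap plays a timeline that sinks the mesh toward the world origin, firing OnPressed when fully down.
; StayPressed switches disable their collision to latch; others use paired DoOnce gates to fire OnUnPressed and reverse the timeline on end overlap.
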(event OnComponentBeginOverlap(Box)
  (params (OverlappedComponent :type Primitive%20Component%20Object%20Reference) (OtherActor :type Actor%20Object%20Reference) (OtherComp :type Primitive%20Component%20Object%20Reference) (OtherBodyIndex :type Integer) (bFromSweep :type Boolean) (SweepResult :type Hit%20Result%20Structure%20%28by%20ref%29))
  (if (Variables|Switch|GetbStayPressed)
    (Collision|SetCollisionEnabled (Variables|Default|GetBox) "NoCollision")
    ;[1 1 1] Lerp switch mesh to pressed state
    (bind (_direction _t) (Timeline|SwitchPressLerp Play)
      (:Update
        (Transformation|SetWorldLocation (Variables|Default|GetStaticMesh) (Math|Vector|Lerp(Vector) (Variables|Default|GetButtonStartLocation) (Variables|Default|GetButtonTargetLocation) _t) false false))
      (:Finished
        (switch Utilities|FlowControl|Switch|SwitchonETimelineDirection _direction
          (:Forward
            (Default|CallOnPressed)))))
    (else
      (Utilities|FlowControl|DoOnce false
        (:Completed
          (Utilities|FlowControl|Sequence
            (:then_0
              (Utilities|FlowControl|DoOnce true) ; enters at Reset
            )
            (:then_1
              (Timeline|SwitchPressLerp Play))))))))

(event OnComponentEndOverlap(Box)
  (params (OverlappedComponent :type Primitive%20Component%20Object%20Reference) (OtherActor :type Actor%20Object%20Reference) (OtherComp :type Primitive%20Component%20Object%20Reference) (OtherBodyIndex :type Integer))
  (Utilities|FlowControl|DoOnce true
    (:Completed
      (Utilities|FlowControl|Sequence
        (:then_0
          (Utilities|FlowControl|DoOnce false) ; enters at Reset
        )
        (:then_1
          (Default|CallOnUnPressed))
        (:then_2
          ;[1 1 1] Lerp switch mesh to pressed state
          (bind (_direction _t) (Timeline|SwitchPressLerp Reverse)
            (:Update
              (Transformation|SetWorldLocation (Variables|Default|GetStaticMesh) (Math|Vector|Lerp(Vector) (Variables|Default|GetButtonStartLocation) (Variables|Default|GetButtonTargetLocation) _t) false false))
            (:Finished
              (switch Utilities|FlowControl|Switch|SwitchonETimelineDirection _direction
                (:Forward
                  (Default|CallOnPressed))))))))))

(event EventBeginPlay
  (bind _output_get (Variables|Default|SetButtonStartLocation (Transformation|GetWorldLocation (Variables|Default|GetStaticMesh))))
  (Variables|Default|SetButtonTargetLocation (+ _output_get (* (Math|Vector|GetUnitDirection(Vector) _output_get "0, 0, 0") (Variables|Switch|GetDistanceMoveOnPressed)))))

(fn ConstructionScript
  (CallFunction|SetActorRotationonSphere self (Variables|Gravity|GetbUpsideDown)))
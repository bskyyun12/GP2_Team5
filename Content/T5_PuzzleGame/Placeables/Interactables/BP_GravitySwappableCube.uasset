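; BP_GravitySwappableCube is a puzzle-game interactable that currently only toggles a point light when clicked.
; BeginPlay applies the Visiable flag to TempPointLight, and ClickInteract flips that flag and updates the light.
; ResetClickInteract clears the flag and hides the light.
; The graph holds no gravity-swapping logic despite the name.
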(event EventBeginPlay
  (Rendering|SetVisibility (Variables|Default|GetTempPointLight) (Variables|Default|GetbVisiable) false))

(event Collision|EventActorBeginOverlap
  (params (OtherActor :type Actor%20Object%20Reference)))

(event EventTick
  (params (DeltaSeconds :type Float%20%28single-precision%29)))

(event EventClickInteract
  (bind _output_get (Variables|Default|SetbVisiable (not (Variables|Default|GetbVisiable))))
  (Rendering|SetVisibility (Variables|Default|GetTempPointLight) _output_get false))

(event EventResetClickInteract
  (bind _output_get (Variables|Default|SetbVisiable false))
  (Rendering|SetVisibility (Variables|Default|GetTempPointLight) _output_get false))

(fn ConstructionScript)
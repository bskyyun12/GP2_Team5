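; Grabbable component that lets the player carry its owning object, typically a BP_GravitySwappableCube, in the gravity puzzle game.
; While grabbed, Tick holds it ahead of the player, tracing toward or away from world origin by gravity state to set surface alignment and height.
; Grab and release toggle the cube's ground collision and physics, plus the character's orient-to-movement.
; The gravity-change binding is disconnected, so GravityChanged is never bound here.
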(event Custom|ReleaseObject
  (bind _returnvalue (Components|GetOwner))
  ;[1 1 1] Get Released
  (Variables|Default|SetbIsGrabbed false)
  (bind _asbp_gravity_swappable_cube (Utilities|Casting|CastToBP_GravitySwappableCube _returnvalue))
  (Default|SetGrondCollision _asbp_gravity_swappable_cube "ECR_Block")
  (Physics|SetSimulatePhysics (Actor|GetComponentbyClass _returnvalue "/Script/Engine.StaticMeshComponent") true)
  (bind _asgravity_character (Utilities|Casting|CastToGravityCharacter (Game|GetPlayerCharacter 0)))
  (Variables|/Script/Engine.CharacterMovementComponent|SetbOrientRotationToMovement (Class|GravityCharacter|GetGravityMovementComponent _asgravity_character) true))

(event Custom|GrabObject
  (bind _returnvalue (Components|GetOwner))
  ;[1 1 1] Get Grabbed
  (Variables|Default|SetbIsGrabbed true)
  (bind _asbp_gravity_swappable_cube (Utilities|Casting|CastToBP_GravitySwappableCube _returnvalue))
  (Default|SetGrondCollision _asbp_gravity_swappable_cube "ECR_Ignore")
  (Physics|SetSimulatePhysics (Actor|GetComponentbyClass _returnvalue "/Script/Engine.StaticMeshComponent") false)
  (bind _asgravity_character (Utilities|Casting|CastToGravityCharacter (Game|GetPlayerCharacter 0)))
  (Variables|/Script/Engine.CharacterMovementComponent|SetbOrientRotationToMovement (Class|GravityCharacter|GetGravityMovementComponent _asgravity_character) false))

(event Custom|GravityChanged
  (params (bInverted :type Boolean))
  (Variables|Default|SetbIsGravityDown (not bInverted)))

(event EventBeginPlay)

(event EventTick
  (params (DeltaSeconds :type Float%20%28single-precision%29))
  (bind _returnvalue (Components|GetOwner))
  (bind _returnvalue_2 (Components|GetOwner))
  (bind _returnvalue_3 (Components|GetOwner))
  (bind _returnvalue_4 (Components|GetOwner))
  (bind _returnvalue_5 (Game|GetPlayerCharacter 0))
  (bind _returnvalue_6 (Game|GetPlayerCharacter 0))
  (bind _returnvalue_7 (Transformation|GetActorRotation _returnvalue_3))
  (bind _returnvalue_8 (Actor|GetComponentbyClass _returnvalue_4 "/Script/Engine.StaticMeshComponent"))
  (bind _capsulecomponent (Variables|/Script/Engine.Character|GetCapsuleComponent _returnvalue_5))
  (bind _rootcomponent (Variables|/Script/Engine.Actor|GetRootComponent _returnvalue_2))
  (bind _rootcomponent_2 (Variables|/Script/Engine.Actor|GetRootComponent _returnvalue))
  (bind _capsulecomponent_2 (Variables|/Script/Engine.Character|GetCapsuleComponent _returnvalue_6))
  (bind _returnvalue_9 (Transformation|GetWorldLocation _returnvalue_8))
  (bind _returnvalue_10 (Transformation|GetWorldLocation _capsulecomponent_2))
  (bind _returnvalue_11 (Math|Vector|GetForwardVector _capsulecomponent))
  (bind _returnvalue_12 (Transformation|GetWorldLocation _capsulecomponent))
  (bind (_roll _pitch _yaw) (Math|Rotator|BreakRotator _returnvalue_7))
  (bind _returnvalue_13 (Math|Vector|GetForwardVector _capsulecomponent_2))
  (bind _returnvalue_14 (* _returnvalue_13 1.2e+02))
  (bind _returnvalue_15 (* _returnvalue_11 1.2e+02))
  (bind _returnvalue_16 (+ _returnvalue_10 _returnvalue_14))
  (bind _returnvalue_17 (+ _returnvalue_12 _returnvalue_15))
  ;[1 1 1] Grabbed Logic
  (if (Variables|Default|GetbIsGrabbed)
    (if (Variables|Default|GetbIsGravityDown)
      (bind _outhit (Collision|LineTraceByChannel (Transformation|GetWorldLocation (Actor|GetComponentbyClass (Components|GetOwner) "/Script/Engine.StaticMeshComponent")) "0, 0, 0" "TraceTypeQuery1" false 0 "ForOneFrame"))
      (Transformation|SetWorldRotation _rootcomponent_2 (Math|Rotator|MakeRotfromZX (.ImpactNormal (Collision|BreakHitResult _outhit)) (Math|Vector|GetForwardVector (Math|Rotator|MakeRotator _roll 0.0 _yaw))) false false)
      (Transformation|SetWorldLocation _rootcomponent_2 (- _returnvalue_16 (* (Math|Vector|GetUpVector (Actor|GetComponentbyClass (Components|GetOwner) "/Script/Engine.StaticMeshComponent")) (- (Math|Vector|Distance(Vector) _returnvalue_16 (.ImpactPoint (Collision|BreakHitResult _outhit))) 65.0))) true false)
      (else
        (bind _outhit_2 (Collision|LineTraceByChannel _returnvalue_9 (* (Math|Vector|GetUnitDirection(Vector) "0, 0, 0" _returnvalue_9) 1e+04) "TraceTypeQuery1" false 0 "ForOneFrame"))
        (Transformation|SetWorldRotation _rootcomponent (Math|Rotator|MakeRotfromZX (.ImpactNormal (Collision|BreakHitResult _outhit_2)) (Math|Vector|GetForwardVector (Variables|/Script/Engine.Character|GetCapsuleComponent (Game|GetPlayerCharacter 0)))) false false)
        (Transformation|SetWorldLocation _rootcomponent (- _returnvalue_17 (* (Math|Vector|GetUpVector (Actor|GetComponentbyClass (Components|GetOwner) "/Script/Engine.StaticMeshComponent")) (- (Math|Vector|Distance(Vector) _returnvalue_17 (.ImpactPoint (Collision|BreakHitResult _outhit_2))) 65.0))) true false)))))
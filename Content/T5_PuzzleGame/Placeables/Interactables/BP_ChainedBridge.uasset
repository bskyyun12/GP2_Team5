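; BP_ChainedBridge is a puzzle-game interactable: a bridge hung on four cables, with click selection shown by a point light.
; The construction script attaches each cable end to its referenced location actor.
; ClickInteract clicks toggle the light and set Selected, while its reset event clears both.
; SetGrondCollision sets the response of four capsules on a custom trace channel, with no caller in this Blueprint.
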(event OnClickInteract(ClickInteract)
  (bind _output_get (Variables|Default|SetbLightOn (not (Variables|Default|GetbLightOn))))
  (Rendering|SetVisibility (Variables|Default|GetTempPointLight) _output_get false)
  (Variables|Default|SetbSelected true))

(event OnResetClickInteract(ClickInteract)
  (bind _output_get (Variables|Default|SetbLightOn false))
  (Rendering|SetVisibility (Variables|Default|GetTempPointLight) _output_get false)
  (Variables|Default|SetbSelected false))

(event EventBeginPlay
  (Rendering|SetVisibility (Variables|Default|GetTempPointLight) (Variables|Default|GetbLightOn) false))

(fn ConstructionScript
  (Class|CableComponent|SetAttachEndto (Variables|Default|GetCable) (Variables|Default|GetCable1Loc) "None" "None")
  (Class|CableComponent|SetAttachEndto (Variables|Default|GetCable1) (Variables|Default|GetCable2Loc) "None" "None")
  (Class|CableComponent|SetAttachEndto (Variables|Default|GetCable2) (Variables|Default|GetCable3Loc) "None" "None")
  (Class|CableComponent|SetAttachEndto (Variables|Default|GetCable3) (Variables|Default|GetCable4Loc) "None" "None"))

(fn SetGrondCollision
  (params (CollisionEnabled :type ECollisionResponse%20Enum :default "ECR_Ignore"))
  (Collision|SetCollisionResponsetoChannel (Variables|Default|GetCapsule) "ECC_GameTraceChannel2" CollisionEnabled))
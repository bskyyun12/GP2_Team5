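; BP_DeathTriggerComponent is a component that handles a death reset for the player in the puzzle game's checkpoint system.
; On BeginPlay it caches references to the player character and BP_RespawnManger.
; Its OnRest event disables the owner's input, waits briefly, loads the save slot, moves the player and re-enables input.
; The move targets the world origin, and neither the loaded save nor the manager reference is used here.
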(event EventBeginPlay
  (bind _returnvalue (Actor|GetActorOfClass 0))
  (Variables|Default|SetPlayerCharacterRefrances _returnvalue)
  (bind _returnvalue_2 (Actor|GetActorOfClass "/Game/T5_PuzzleGame/Placeables/CheckpointSystem/BP_RespawnManger.BP_RespawnManger_C"))
  (Variables|Default|SetRespawnManger _returnvalue_2))

(event EventOnRest
  (bind _playercharacterrefrances (Variables|Default|GetPlayerCharacterRefrances))
  (Input|DisableInput (Components|GetOwner) 0)
  (Utilities|FlowControl|Delay 2.0)
  (SaveGame|LoadGamefromSlot (Variables|Default|GetSaveSlot))
  (Transformation|SetActorLocation _playercharacterrefrances "0, 0, 0" false false)
  (Input|EnableInput _playercharacterrefrances (Game|GetPlayerController 0)))
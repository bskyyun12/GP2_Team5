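; BP_RespawnData is a component that stores reset state for its owning actor in the puzzle game's checkpoint system.
; It records the owner's starting transform on BeginPlay and saves the GravitySwapComponent's FlipGravity state, if that component exists, when OnEnterCheckPoint fires.
; OnRest returns the owner to that starting transform, which checkpoints never update, and restores the saved gravity flip without a validity check.
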(event EventBeginPlay
  (Variables|Default|SetStartActorLocation (Transformation|GetActorTransform (Components|GetOwner))))

(event EventOnRest
  (Transformation|SetActorTransform (Components|GetOwner) (Variables|Default|GetStartActorLocation))
  (Variables|/Script/GP2_Team5.GravitySwapComponent|SetbFlipGravity (Actor|GetComponentbyClass (Components|GetOwner) "/Script/GP2_Team5.GravitySwapComponent") (Variables|Default|GetFlipGravitySave)))

(event EventOnEnterCheckPoint
  (params (Caller :type Actor%20Object%20Reference))
  (bind _returnvalue (Components|GetOwner))
  (bind _returnvalue_2 (Actor|GetComponentbyClass _returnvalue "/Script/GP2_Team5.GravitySwapComponent"))
  (Utilities|IsValid _returnvalue_2
    (:Is%20Valid
      (Variables|Default|SetFlipGravitySave (Variables|/Script/GP2_Team5.GravitySwapComponent|GetbFlipGravity _returnvalue_2)))))
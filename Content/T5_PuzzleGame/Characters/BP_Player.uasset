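; Player character for the puzzle game, whose only active logic is a camera zoom on Left Shift.
; Pressing and releasing Shift finds the first BP_FollowCamera via GetAllActorsOfClass and switches it between zoomed and normal view.
; OnRest and OnEnterCheckPoint are empty events.
; Unconnected nodes would save and restore the GravitySwap flip state, call OnRest on the death trigger component and zero movement velocity, but never run.
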(event EventBeginPlay
  (|CallParentFunction) ; This node is disabled and will not be called.\nDrag off pins to build functionality.
)

(event Collision|EventActorBeginOverlap
  (params (OtherActor :type Actor%20Object%20Reference)))

(event EventTick
  (params (DeltaSeconds :type Float%20%28single-precision%29))
  (|CallParentFunction DeltaSeconds) ; This node is disabled and will not be called.\nDrag off pins to build functionality.
)

(event EventOnRest)

(event EventOnEnterCheckPoint
  (params (Caller :type Actor%20Object%20Reference)))

(event Input|KeyboardEvents|LeftShift
  (params (Key :type Key%20Structure :default "None"))
  (:Pressed
    (bind _outactors (Actor|GetAllActorsOfClass "/Game/T5_PuzzleGame/BP_FollowCamera.BP_FollowCamera_C"))
    (Default|ZoomedView (Utilities|Array|Get(acopy) _outactors)))
  (:Released
    (bind _outactors_2 (Actor|GetAllActorsOfClass "/Game/T5_PuzzleGame/BP_FollowCamera.BP_FollowCamera_C"))
    (Default|NormalVieqw (Utilities|Array|Get(acopy) _outactors_2))))

(fn ConstructionScript
  (|CallParentFunction))
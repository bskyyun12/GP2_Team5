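; Player character for a puzzle game with flippable gravity, click interaction and a death trigger component.
; Sets its starting gravity at BeginPlay, then negates the camera boom's socket offset whenever the GravitySwap component reports an inverted flip.
; Temporary lights show state: one is recolored each tick by gravity direction, the other toggles with ClickInteract events.
; OnRest is forwarded to the death trigger component.
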(event OnClickInteract(ClickInteract)
  ;[1 1 1] Temporary stuff
  (bind _output_get (Variables|Default|SetbClicked (not (Variables|Default|GetbClicked))))
  (Rendering|SetVisibility (Variables|Default|GetTempClickedLight) _output_get false))

(event OnResetClickInteract(ClickInteract)
  ;[1 1 1] Temporary stuff
  (bind _output_get (Variables|Default|SetbClicked false))
  (Rendering|SetVisibility (Variables|Default|GetTempClickedLight) _output_get false))

(event OnFlipGravity(GravitySwap)
  (params (bInverted :type Boolean))
  (bind _cameraboom (Variables|Default|GetCameraBoom))
  (bind _cameraboomdefaultoffset (Variables|Default|GetCameraBoomDefaultOffset))
  ;[1 1 1] On Flip Gravity :  Change camera focus when gravity flips
  (bind _output_get (Variables|Default|SetbFlipGravity bInverted))
  (if _output_get
    (Variables|/Script/Engine.SpringArmComponent|SetSocketOffset _cameraboom (* _cameraboomdefaultoffset -1.0))
    (else
      (Variables|/Script/Engine.SpringArmComponent|SetSocketOffset _cameraboom _cameraboomdefaultoffset))))

(event EventBeginPlay
  (Class|GravityCharacter|SetGravityTarget (Variables|Default|GetStartGravity))
  (Variables|Default|SetCameraBoomDefaultOffset (Variables|/Script/Engine.SpringArmComponent|GetSocketOffset (Variables|Default|GetCameraBoom))))

(event EventOnRest
  ;[1 1 1] Comment
  (Class|CheckPointInterface|OnRest (Variables|Default|GetBP_DeathTriggerComponent)))

(event EventTick
  (params (DeltaSeconds :type Float%20%28single-precision%29))
  ;[1 1 1] Temporary stuff
  (if (Variables|Default|GetbFlipGravity)
    (Rendering|Components|Light|SetLightColor (Variables|Default|GetTempCharacterLight) (Variables|Default|GetBlueLight) true)
    (else
      (Rendering|Components|Light|SetLightColor (Variables|Default|GetTempCharacterLight) (Variables|Default|GetRedLight) true))))

(event Input|KeyboardEvents|X
  (params (Key :type Key%20Structure :default "None")))

(fn ConstructionScript)
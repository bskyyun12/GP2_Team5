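; Follow camera for the puzzle game that tracks the first BP_Player side-on and rolls with them around the world origin.
; Each tick, a trace along the player's down axis finds the ground, and the camera eases toward an offset above it in Y/Z, with X set by Zoom.
; Its rotation eases to treat the origin-to-player direction as up, with yaw fixed to face along negative X.
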(event EventTick
  (params (DeltaSeconds :type Float%20%28single-precision%29))
  (bind _playercharacter (Variables|Default|GetPlayerCharacter))
  (bind _playercharacter_2 (Variables|Default|GetPlayerCharacter))
  (bind _returnvalue (Transformation|GetActorUpVector _playercharacter_2))
  (bind _capsulecomponent (Variables|/Script/Engine.Character|GetCapsuleComponent _playercharacter))
  (bind _returnvalue_2 (Transformation|GetWorldLocation _capsulecomponent))
  (bind _returnvalue_3 (Math|Vector|GetUnitDirection(Vector) "0, 0, 0" _returnvalue_2))
  (bind _returnvalue_4 (Math|Vector|RotateVector _returnvalue_3 "0, 0,-90.000000"))
  (bind _returnvalue_5 (Class|KismetMathLibrary|MakeRotfromYZ _returnvalue_4 _returnvalue_3))
  (bind (_roll _pitch) (Math|Rotator|BreakRotator _returnvalue_5))
  (bind _outhit (Collision|LineTraceByChannel (Transformation|GetActorLocation _playercharacter_2) (* _returnvalue -1e+05) "TraceTypeQuery3" false 0 "None"))
  (Transformation|SetWorldLocation (Variables|CameraActor|GetCameraComponent) (Math|Interpolation|VInterpTo (Transformation|GetWorldLocation (Variables|CameraActor|GetCameraComponent)) (Math|Vector|MakeVector (Variables|Default|Getzoom) (.Y (Math|Vector|BreakVector (+ (.Location (Collision|BreakHitResult _outhit)) (* _returnvalue (Variables|Default|GetOffset))))) (.Z (Math|Vector|BreakVector (+ (.Location (Collision|BreakHitResult _outhit)) (* _returnvalue (Variables|Default|GetOffset)))))) (Utilities|Time|GetWorldDeltaSeconds) 1e+01) false false)
  (Transformation|SetWorldRotation (Variables|CameraActor|GetCameraComponent) (Math|Interpolation|RInterpTo (Transformation|GetWorldRotation (Variables|CameraActor|GetCameraComponent)) (Math|Rotator|MakeRotator _roll _pitch 1.8e+02) (Utilities|Time|GetWorldDeltaSeconds) 1e+01) false false))

(event EventBeginPlay
  (bind _outactors (Actor|GetAllActorsOfClass "/Game/T5_PuzzleGame/Characters/BP_Player.BP_Player_C"))
  (Variables|Default|SetPlayerCharacter (Utilities|Array|Get(acopy) _outactors)))

(fn ConstructionScript)